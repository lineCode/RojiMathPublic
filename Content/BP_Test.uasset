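; Test actor that draws a circle-of-life point pattern as instanced static meshes with animated colors.
; ResetCircles generates points with a seeded random circle count, then builds one instanced mesh component and dynamic material per level, read from each point's Z.
; Tick shifts a random-color palette through the levels, periodically reversing direction, to cycle colors across the pattern.
; BeginPlay is empty; debug drawing and instance-removal helpers are also included.
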(event `self.ReceiveBeginPlay`)

(event `ResetCircles`
  (bind (_circlelocations _outpoints) (`RojiMathUtilitiesBPLibrary.CreateCircleOfLifePoints` (* (`KismetMathLibrary.RandomIntegerInRangeFromStream` 6 10 (`self.Stream`)) 2) 200.0 3 3))
  (`|ExecutionSequence`
    (:`then_0`
      (set `self.Points1` _circlelocations))
    (:`then_1`
      (set `self.Points2` _outpoints))
    (:`then_2`
      (`self.CreateMeshInstances`))
    (:`then_3`
      (`self.CreateStaticMeshes`))
    (:`then_4`
      (`self.GenerateColors`))
    (:`then_5`
      (`self.SetColors`))))

(event `RemoveMeshInstances`
  (for (_array_element _array_index) (`self.InstancesCount`)
    (for _index (range (+ _array_element 1))
      (`KismetArrayLibrary.Array_Set` (`self.InstancesToDelete`) _index _index true))
    (`InstancedStaticMeshComponent.RemoveInstances` (`|GetArrayItem` (`self.InstancedStaticMeshes`) _array_index) (`self.InstancesToDelete`))
    (set `self.InstancesToDelete` (`self.Empty`)))
  (set `self.InstancesCount` (`self.Empty`)))

(event `CreateMeshInstances`
  (`|ExecutionSequence`
    (:`then_0`
      (for _array_element (`self.Points2`)
        (set `self.Levels` (`KismetMathLibrary.Max` (`KismetMathLibrary.FTrunc` (.z _array_element)) (`self.Levels`)))))
    (:`then_1`
      (for _index (range (+ (`self.Levels`) 1))
        (set `self.Index` _index)
        (bind _returnvalue (`AddComponent|NODE_AddInstancedStaticMeshComponent-0`))
        (bind _output_get (set `self.InstancedStaticMesh` _returnvalue))
        (`KismetArrayLibrary.Array_Set` (`self.InstancedStaticMeshes`) (`self.Index`) _output_get true)
        (`StaticMeshComponent.SetStaticMesh` (`self.InstancedStaticMesh`) (`|GetArrayItem` (`self.StaticMeshes`) (`self.Index`)))
        (bind _returnvalue_2 (`PrimitiveComponent.CreateDynamicMaterialInstance` (`self.InstancedStaticMesh`) 0 (`self.Source Material`) "None"))
        (`/Engine/EditorBlueprintResources/StandardMacros.IsValid` _returnvalue_2
          (:`Is Valid`
            (`KismetArrayLibrary.Array_Set` (`self.Materials`) (`self.Index`) _returnvalue_2 true)
            (`PrimitiveComponent.SetMaterial` (`self.InstancedStaticMesh`) 0 _returnvalue_2) ; Not needed???
          ))))))

(event `CreateStaticMeshes`
  (bind _scale (`self.Scale`))
  (for _array_element (`self.Points2`)
    (bind _returnvalue (`KismetMathLibrary.FTrunc` (- (.z _array_element) 1.0)))
    (bind _returnvalue_2 (`InstancedStaticMeshComponent.AddInstance` (`|GetArrayItem` (`self.InstancedStaticMeshes`) _returnvalue) (`KismetMathLibrary.MakeTransform` (`KismetMathLibrary.TransformLocation` (`self.GetTransform`) (`KismetMathLibrary.MakeVector` (.x _array_element) (.y _array_element))) (struct) (`KismetMathLibrary.MakeVector` _scale _scale _scale)) true))
    (`KismetArrayLibrary.Array_Set` (`self.InstancesCount`) _returnvalue _returnvalue_2 true)))

(event `GenerateColors`
  (for _index (range (+ (`self.Levels`) 1))
    (bind _color (`self.GetRandomColor`))
    (`KismetArrayLibrary.Array_Set` (`self.Colors`) _index _color true)))

(event `self.ReceiveTick`
  (params (DeltaSeconds :type "Float (single-precision)"))
  (`|ExecutionSequence`
    (:`then_0`
      (bind _result (`/Engine/EditorBlueprintResources/StandardMacros.IncrementInt` (`self.Counter`))
        (:`  `
          (if (> _result (* (`self.Levels`) (`self.Loops`)))
            (if (> (`self.Counter`) (* (`self.Levels`) (* (`self.Loops`) 2)))
              (set `self.Counter` 0)
              (else
                (`self.AdjustColors`)))
            (else
              (`self.AdjustColors2`))))))
    (:`then_1`
      (`self.SetColors`))))

(event `SetColors`
  (bind _colors (`self.Colors`))
  (bind _materials (`self.Materials`))
  (for _index (range (+ (`self.Levels`) 1))
    (if (and (> (`KismetArrayLibrary.Array_Length` _materials) _index) (> (`KismetArrayLibrary.Array_Length` _colors) _index))
      (bind _output (`|GetArrayItem` _materials _index))
      (`MaterialInstanceDynamic.SetVectorParameterValue` _output "Color" (`|GetArrayItem` _colors _index))
      (`PrimitiveComponent.SetMaterial` (`|GetArrayItem` (`self.InstancedStaticMeshes`) _index) 0 _output))))

(event `ShowDebugMarkers`
  (`/Engine/EditorBlueprintResources/StandardMacros.IncrementInt` (`self.Counter`)
    (:`  `
      (for _array_element (`self.Points2`)
        (`|ExecutionSequence`
          (:`then_0`
            (`|ExecutionSequence`
              (:`then_0`
                (bind _returnvalue (`KismetMathLibrary.FTrunc` (.z _array_element)))
                (if (!= (mod _returnvalue 2) 0)
                  _
                  (else
                    _))
                (set `self.ColorNumber` (- 7 (mod (+ _returnvalue (`self.Counter`)) 8))))
              (:`then_1`
                (switch `int` (`self.ColorNumber`)
                  (:`0`
                    (set `self.MarkerColor` (struct :`R` 0.41813 :`G` 0.370998 :`B` 1.0 :`A` 1.0)))
                  (:`1`
                    (set `self.MarkerColor` (struct :`R` 0.810359 :`B` 1.0 :`A` 1.0)))
                  (:`2`
                    (set `self.MarkerColor` (struct :`R` 0.070491 :`G` 1.0 :`B` 0.35213 :`A` 1.0)))
                  (:`3`
                    (set `self.MarkerColor` (struct :`R` 1.0 :`G` 0.473848 :`B` 0.023872 :`A` 1.0)))
                  (:`4`
                    (set `self.MarkerColor` (struct :`R` 0.057076 :`G` 0.748045 :`B` 1.0 :`A` 1.0)))
                  (:`5`
                    (set `self.MarkerColor` (struct :`R` 0.905365 :`G` 1.0 :`A` 1.0)))
                  (:`6`
                    (set `self.MarkerColor` (struct :`R` 0.300997 :`G` 0.013079 :`B` 1.0 :`A` 1.0)))
                  (:`7`
                    (set `self.MarkerColor` (struct :`R` 1.0 :`G` 0.17521 :`A` 1.0)))))))
          (:`then_1`
            (`KismetSystemLibrary.DrawDebugPoint` (`KismetMathLibrary.MakeVector` (.x _array_element) (.y _array_element) 50.0) 10.0 (`self.MarkerColor`) (`self.Time`))))))))

(event `AdjustColors`
  (bind _colors (`self.Colors`))
  (bind _color (`self.GetRandomColor`))
  (set `self.Color0` _color)
  (for _index (range (+ (`self.Levels`) 1))
    (if (== _index (`self.Levels`))
      (`KismetArrayLibrary.Array_Set` (`self.Colors`) _index (`self.Color0`))
      (else
        (`KismetArrayLibrary.Array_Set` _colors _index (`|GetArrayItem` _colors (+ _index 1)))))))

(event `AdjustColors2`
  (bind _colors (`self.Colors`))
  (bind _color (`self.GetRandomColor`))
  (set `self.Color0` _color)
  (bind _output_get (set `self.Index` (`self.Levels`)))
  (while (>= _output_get 0)
    (`|ExecutionSequence`
      (:`then_0`
        (if (== (`self.Index`) 0)
          (`KismetArrayLibrary.Array_Set` (`self.Colors`) 0 (`self.Color0`))
          (else
            (`KismetArrayLibrary.Array_Set` _colors (`self.Index`) (`|GetArrayItem` _colors (- (`self.Index`) 1))))))
      (:`then_1`
        (`/Engine/EditorBlueprintResources/StandardMacros.DecrementInt` (`self.Index`))))))

(fn `GetRandomColor`
  (returns (Color :type "LinearColor Structure"))
  (bind _stream (`self.Stream`))
  (return (make `LinearColor` (`KismetMathLibrary.RandomFloatInRangeFromStream` 0.0 1.0 _stream) (`KismetMathLibrary.RandomFloatInRangeFromStream` 0.0 1.0 _stream) (`KismetMathLibrary.RandomFloatInRangeFromStream` 0.0 1.0 _stream) 1.0)))

(fn `ShowMarkers`
  (params (InPoints1 :type "Array of Vector Structure (by ref)") (InPoints2 :type "Array of Vector Structure") (IntPoints :type "Array of IntPoint Structure"))
  (locals (Radius :type "Float (double-precision)" :default 7.0) (Color :type "LinearColor Structure" :default (struct :`G` 1.0 :`B` 1.0 :`A` 1.0)) (Duration :type "Float (double-precision)" :default 999.0) (Thickness :type "Float (double-precision)" :default 10.0))
  (`|ExecutionSequence`
    (:`then_0`
      (for (_array_element _array_index) InPoints1
        (`KismetSystemLibrary.DrawDebugLine` _array_element (`|GetArrayItem` InPoints2 _array_index) (`local.Color`) (`local.Duration`) (`local.Thickness`))))
    (:`then_1`
      (for _array_element_2 IntPoints
        (bind (_output_x _output_y) (`KismetMathLibrary.BreakVector` (`|GetArrayItem` InPoints1 (`.Y` (break `IntPoint` _array_element_2)))))
        (bind _returnvalue (/ (`KismetMathLibrary.Sqrt` (+ (`KismetMathLibrary.Square` _output_x) (`KismetMathLibrary.Square` _output_y))) 10000.0))
        (`KismetSystemLibrary.DrawDebugLine` (`|GetArrayItem` InPoints1 (`.Y` (break `IntPoint` _array_element_2))) (`|GetArrayItem` InPoints2 (`.Y` (break `IntPoint` _array_element_2))) (make `LinearColor` _returnvalue (- 1.0 _returnvalue)) 999.0 50.0)))))

(fn `UserConstructionScript`)