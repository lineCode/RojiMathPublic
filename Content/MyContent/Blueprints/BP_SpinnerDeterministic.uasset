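; BP_SpinnerDeterministic scatters repeatable instanced copies of a static mesh within a spherical radius around the actor.
; UseConstructor selects whether the instanced mesh component, with optional dynamic material, is built in the Construction Script or at BeginPlay, using duplicated logic.
; A random stream set from DeterministicID drives each instance's position, yaw and per-axis scale variation.
; Positions combine a normalized random direction with cube-root radial distribution; no spinning logic appears here.
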(event `self.ReceiveBeginPlay`
  (bind _returnvalue (`self.GetTransform`))
  (bind _returnvalue_2 (- (`self.Instances`) 1))
  (if (not (`self.UseConstructor`))
    (`|ExecutionSequence`
      (:`then_0`
        ;[1 1 1] Create Instance
        (bind _returnvalue_3 (`AddComponent|NODE_AddInstancedStaticMeshComponent-3`))
        (bind _output_get (set `self.InstancedStaticMesh` _returnvalue_3))
        (`StaticMeshComponent.SetStaticMesh` _output_get (`self.StaticMesh`))
        (if (`self.UseMaterial`)
          (bind _returnvalue_4 (`PrimitiveComponent.CreateDynamicMaterialInstance` (`self.InstancedStaticMesh`) 0 (`self.Source Material`) "None"))
          (`PrimitiveComponent.SetMaterial` (`self.InstancedStaticMesh`) 0 _returnvalue_4)))
      (:`then_1`
        (set `self.Stream` (`KismetMathLibrary.MakeRandomStream` (`self.DeterministicID`))))
      (:`then_2`
        (if (>= _returnvalue_2 0)
          (for _ (range (+ _returnvalue_2 1))
            (bind (_x _y _z) (`self.GetRandomPointInSphere`))
            (bind (_returnvalue_5 _returnvalue2 _returnvalue3) (`self.GetRandomScale`))
            (`InstancedStaticMeshComponent.AddInstance` (`self.InstancedStaticMesh`) (`KismetMathLibrary.MakeTransform` (`KismetMathLibrary.TransformLocation` _returnvalue (`KismetMathLibrary.MakeVector` _x _y _z)) (`KismetMathLibrary.TransformRotation` _returnvalue (`KismetMathLibrary.MakeRotator` 0.0 0.0 (`KismetMathLibrary.RandomFloatInRangeFromStream` 0.0 360.0 (`self.Stream`)))) (`KismetMathLibrary.MakeVector` _returnvalue_5 _returnvalue2 _returnvalue3)) true)))))))

(fn `GetRandomPointInSphere`
  (returns (X :type "Float (double-precision)") (Y :type "Float (double-precision)") (Z :type "Float (double-precision)"))
  (locals (XX :type "Float (double-precision)") (YY :type "Float (double-precision)") (ZZ :type "Float (double-precision)") (U :type "Float (double-precision)") (Mag :type "Float (double-precision)"))
  (set `local.U` (`KismetMathLibrary.MultiplyMultiply_FloatFloat` (`KismetMathLibrary.RandomFloatFromStream` (`self.Stream`)) 0.333333))
  (set `local.XX` (`KismetMathLibrary.RandomFloatInRangeFromStream` -1.0 1.0 (`self.Stream`)))
  (set `local.YY` (`KismetMathLibrary.RandomFloatInRangeFromStream` -1.0 1.0 (`self.Stream`)))
  (set `local.ZZ` (`KismetMathLibrary.RandomFloatInRangeFromStream` -1.0 1.0 (`self.Stream`)))
  (set `local.Mag` (`KismetMathLibrary.Sqrt` (+ (`KismetMathLibrary.Square` (`local.XX`)) (`KismetMathLibrary.Square` (`local.YY`)) (`KismetMathLibrary.Square` (`local.ZZ`)))))
  (return (* (* (`local.U`) (/ (`local.XX`) (`local.Mag`))) (`self.Radius`)) (* (* (`local.U`) (/ (`local.YY`) (`local.Mag`))) (`self.Radius`)) (* (* (`local.U`) (/ (`local.ZZ`) (`local.Mag`))) (`self.Radius`))))

(fn `GetRandomScale`
  (returns (ReturnValue :type "Float (double-precision)") (ReturnValue2 :type "Float (double-precision)") (ReturnValue3 :type "Float (double-precision)"))
  (bind _returnvalue (`self.GetTransform`))
  (bind _deltascale (`self.DeltaScale`))
  (bind _returnvalue_2 (* _deltascale -1.0))
  (return (+ (.x (.scale _returnvalue)) (* (.x (.scale _returnvalue)) (`KismetMathLibrary.RandomFloatInRangeFromStream` _returnvalue_2 _deltascale (`self.Stream`)))) (+ (.y (.scale _returnvalue)) (* (.y (.scale _returnvalue)) (`KismetMathLibrary.RandomFloatInRangeFromStream` _returnvalue_2 _deltascale (`self.Stream`)))) (+ (.z (.scale _returnvalue)) (* (.z (.scale _returnvalue)) (`KismetMathLibrary.RandomFloatInRangeFromStream` _returnvalue_2 _deltascale (`self.Stream`))))))

(fn `UserConstructionScript`
  (bind _returnvalue (`self.GetTransform`))
  (bind _returnvalue_2 (- (`self.Instances`) 1))
  (if (`self.UseConstructor`)
    (`|ExecutionSequence`
      (:`then_0`
        ;[1 1 1] Create Instance
        (bind _returnvalue_3 (`AddComponent|NODE_AddInstancedStaticMeshComponent-2`))
        (bind _output_get (set `self.InstancedStaticMesh` _returnvalue_3))
        (`StaticMeshComponent.SetStaticMesh` _output_get (`self.StaticMesh`))
        (if (`self.UseMaterial`)
          (bind _returnvalue_4 (`PrimitiveComponent.CreateDynamicMaterialInstance` (`self.InstancedStaticMesh`) 0 (`self.Source Material`) "None"))
          (`PrimitiveComponent.SetMaterial` (`self.InstancedStaticMesh`) 0 _returnvalue_4)))
      (:`then_1`
        (set `self.Stream` (`KismetMathLibrary.MakeRandomStream` (`self.DeterministicID`))))
      (:`then_2`
        (if (>= _returnvalue_2 0)
          (for _ (range (+ _returnvalue_2 1))
            (bind (_x _y _z) (`self.GetRandomPointInSphere`))
            (bind (_returnvalue_5 _returnvalue2 _returnvalue3) (`self.GetRandomScale`))
            (`InstancedStaticMeshComponent.AddInstance` (`self.InstancedStaticMesh`) (`KismetMathLibrary.MakeTransform` (`KismetMathLibrary.TransformLocation` _returnvalue (`KismetMathLibrary.MakeVector` _x _y _z)) (`KismetMathLibrary.TransformRotation` _returnvalue (`KismetMathLibrary.MakeRotator` 0.0 0.0 (`KismetMathLibrary.RandomFloatInRangeFromStream` 0.0 360.0 (`self.Stream`)))) (`KismetMathLibrary.MakeVector` _returnvalue_5 _returnvalue2 _returnvalue3)) true)))))))