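; Test actor that exercises polygon-to-triangle and grid-fill geometry helpers and visualizes the results.
; On BeginPlay it adds the Points polygon to the A/B/C triangle data, then replaces Points with the output of CreateGridInLayer, using Spacing and Depth.
; ShowMarkers draws the points, triangle layer and bounding box in the actor's transform.
; The construction script is empty; open-polygon and triangle-merging experiments remain unconnected in both graphs.
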(event `self.ReceiveBeginPlay`
  (`|ExecutionSequence`
    (:`then_0`
      (bind (_outa _outb _outc) (`RojiMathUtilitiesBPLibrary.AddPolygonToTriangles` (`self.Points`) (`self.A`) (`self.B`) (`self.C`)))
      (`|ExecutionSequence`
        (:`then_0`
          (set `self.A` _outa))
        (:`then_1`
          (set `self.B` _outb))
        (:`then_2`
          (set `self.C` _outc))))
    (:`then_2`
      (bind _outpoints (`RojiMathUtilitiesBPLibrary.CreateGridInLayer` (`self.Points`) (`self.A`) (`self.B`) (`self.C`) (`self.Spacing`) (`self.Depth`)))
      (bind _output_get (set `self.Points` _outpoints))
      (`self.ShowMarkers` _output_get))))

(fn `ShowMarkers`
  (params (InPoints :type "Array of Vector Structure (by ref)"))
  (locals (Radius :type "Float (double-precision)" :default 7.0) (Color :type "LinearColor Structure" :default (struct :`R` 1.0 :`G` 0.072683 :`B` 0.873928 :`A` 1.0)) (Duration :type "Float (double-precision)" :default 90.0) (Thickness :type "Float (double-precision)" :default 2.0) (ZOffset :type "Float (double-precision)" :default 50.0))
  (bind _returnvalue (`self.GetTransform`))
  (bind _duration (`local.Duration`))
  (bind _thickness (`local.Thickness`))
  (bind _returnvalue_2 (`KismetMathLibrary.Conv_LinearColorToColor` (`local.Color`)))
  (`|ExecutionSequence`
    (:`then_0`
      (`RojiMathUtilitiesBPLibrary.DrawMarkers` _returnvalue InPoints (`local.Radius`) _returnvalue_2 _duration _thickness)
      (`RojiMathUtilitiesBPLibrary.DrawLayer` _returnvalue (`self.A`) (`self.B`) (`self.C`) (`local.ZOffset`) _returnvalue_2 _duration _thickness)
      (`RojiMathUtilitiesBPLibrary.DrawBoundingBox` _returnvalue (`self.A`) (`self.B`) (`self.C`) (`self.ZZOffset`) (`KismetMathLibrary.Conv_LinearColorToColor` (`self.Color1`)) (`local.Duration`) (`local.Thickness`)))))

(fn `UserConstructionScript`)