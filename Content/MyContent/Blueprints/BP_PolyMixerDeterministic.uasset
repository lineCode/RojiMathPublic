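; BP_PolyMixerDeterministic scatters layered instanced static meshes inside a polygon, then grows them over time and can turn them toward an actor.
; The polygon is fan-triangulated, and each triangle gets instances by area share and layer percentage.
; A seeded stream drives uniform point placement and scale, though random yaw is unseeded.
; Generation runs at construction or BeginPlay; Tick updates one random or all instances per growing layer, with an optional debug fence.
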(event `self.ReceiveBeginPlay`
  (if (not (`self.UseConstructor`))
    (`KismetSystemLibrary.Delay` 0.2)
    (`|ExecutionSequence`
      (:`then_0`
        ;[1 1 1] Create Triangles from Polygon and set area, percentage and count
        (`self.MakeTrianglesFromPolygon`)
        (`self.SetTriangleProperties`)
        (set `self.Stream` (`KismetMathLibrary.MakeRandomStream` (`self.StreamInitialSeed`))))
      (:`then_1`
        ;[1 1 1] Show Debug Fence
        (if (`self.ShowDebugFence`)
          (`self.ShowDebugOutline`)))
      (:`then_2`
        ;[1 1 1] Make the Mesh Instances and individual Meshes in the Triangles
        (if (not (`self.HideMeshes`))
          (`self.MakeMeshInstance`)
          (`self.FillTrianglesWithMeshes`)))
      (:`then_3`
        ;[1 1 1] Start timers for updating Debug Fence and Mesh Manipulation over time
        (`KismetSystemLibrary.K2_SetTimerDelegate` (delegate `UpdateDebugFence`) (`self.DebugDuration`) true :!label _label)
        (set `self.Ready` true)))
    (else
      (goto _label))))

(event `UpdateDebugFence`
  (if (`self.ShowDebugFence`)
    (`self.ShowDebugOutline`)))

(event `Grow`
  (`self.Grow Next Instance` :!label _label_2))

(event `self.ReceiveTick`
  (params (DeltaSeconds :type "Float (single-precision)"))
  (if (`self.Ready`)
    (goto _label_2)))

(fn `FillTrianglesWithMeshes`
  (locals (Rotator :type "Rotator Structure" :default (struct)) (Location :type "Vector Structure" :default (0.0 0.0 0.0)) (CenterLocation :type "Vector Structure") (MinLocation :type "Vector Structure") (MaxLocation :type "Vector Structure") (Min :type "Float (double-precision)") (Max :type "Float (double-precision)") (LookLocation :type "Vector Structure") (ScaleSize :type "Float (double-precision)") (StaticMeshInstance :type "InstancedStaticMeshComponent Object Reference") (Rotation :type "/Game/MyContent/Blueprints/E_RotationType Enum") (PercentageThisMesh :type "Float (double-precision)") (MeshIndex :type Integer) (PolyDetailItem :type "/Game/MyContent/Blueprints/S_InstanceDetails Structure") (MeshCreateIndex :type Integer) (InstanceIndex :type Integer) (DeltaInitialSize :type "Float (double-precision)") (GrowthRate :type "Float (double-precision)"))
  (bind (_returnvalue_x _returnvalue_y _returnvalue_z) (`KismetMathLibrary.BreakVector` (`self.K2_GetActorLocation`)))
  (bind (_returnvalue_x_2 _returnvalue_y_2 _returnvalue_z_2) (`KismetMathLibrary.BreakVector` (`self.K2_GetActorLocation`)))
  (bind (_minlocation_x _minlocation_y) (`KismetMathLibrary.BreakVector` (`local.MinLocation`)))
  (bind (_maxlocation_x _maxlocation_y) (`KismetMathLibrary.BreakVector` (`local.MaxLocation`)))
  (bind _polygon (`self.Polygon`))
  (bind (_looklocation_x _looklocation_y) (`KismetMathLibrary.BreakVector` (`local.LookLocation`)))
  (bind _rotator (`local.Rotator`))
  (bind _instancedetails (`self.InstanceDetails`))
  (bind _meshindex (`local.MeshIndex`))
  (bind _location (`local.Location`))
  (bind _meshcreateindex (`local.MeshCreateIndex`))
  (bind (_minlocation_x_2 _minlocation_y_2) (`KismetMathLibrary.BreakVector` (`local.MinLocation`)))
  (bind (_maxlocation_x_2 _maxlocation_y_2) (`KismetMathLibrary.BreakVector` (`local.MaxLocation`)))
  (bind _returnvalue (`KismetArrayLibrary.Array_Length` (`self.InstancedStaticMesh`)))
  (bind (_returnvalue_roll _returnvalue_pitch _returnvalue_yaw) (`KismetMathLibrary.BreakRotator` (`KismetMathLibrary.FindLookAtRotation` (`local.Location`) (`local.CenterLocation`))))
  (bind (_output_staticmesh _output_sizemin _output_sizemax _output_usematerial _output_materialinstance _output_rotationtype _output_lookatlocation _output_percentagethismesh _output_deltainitialsize _output_growthrate _output_hidemeshes) (break `/Game/MyContent/Blueprints/S_PolyDef` (`|GetArrayItem` (`self.MeshLayers`) (`local.MeshIndex`))))
  (bind _output (`|GetArrayItem` _polygon))
  (bind _returnvalue_2 (* (`local.Min`) (`local.DeltaInitialSize`)))
  (bind (_name _transform _size _ratio) (break `/Game/MyContent/Blueprints/S_InstanceDetails` (`|GetArrayItem` (`self.InstanceDetails`) (`local.MeshIndex`))))
  (bind (_returnvalue_roll_2 _returnvalue_pitch_2 _returnvalue_yaw_2) (`KismetMathLibrary.BreakRotator` (`KismetMathLibrary.FindLookAtRotation` (`local.Location`) (`KismetMathLibrary.MakeVector` _looklocation_x _looklocation_y _returnvalue_z_2))))
  (bind _returnvalue_3 (`KismetMathLibrary.RandomFloatInRangeFromStream` (- (`local.Min`) _returnvalue_2) (+ (`local.Min`) _returnvalue_2) (`self.Stream`)))
  (bind _returnvalue_4 (`KismetMathLibrary.Conv_DoubleToVector` _returnvalue_3))
  ;[1 1 1] Setup
  (if (> _returnvalue 0)
    (for _index (range _returnvalue)
      (set `local.MeshIndex` _index)
      (set `local.StaticMeshInstance` (`|GetArrayItem` (`self.InstancedStaticMesh`) (`local.MeshIndex`)))
      (if (not _output_hidemeshes)
        (set `local.Min` _output_sizemin)
        (set `local.Rotation` _output_rotationtype)
        (set `local.Max` _output_sizemax)
        (set `local.LookLocation` _output_lookatlocation)
        (set `local.PercentageThisMesh` _output_percentagethismesh)
        (set `local.DeltaInitialSize` _output_deltainitialsize)
        (set `local.GrowthRate` _output_growthrate)
        (`|ExecutionSequence`
          (:`then_0`
            ;[1 1 1] Find "Center" of polygon
            (if (`|EnumEquality` (`local.Rotation`) "NewEnumerator3")
              (if (> (`KismetArrayLibrary.Array_Length` _polygon) 0)
                (set `local.MinLocation` _output)
                (set `local.MaxLocation` _output)
                (for _array_element (`self.Polygon`)
                  (set `local.MinLocation` (`KismetMathLibrary.MakeVector` (`KismetMathLibrary.FMin` _minlocation_x (.x _array_element)) (`KismetMathLibrary.FMin` _minlocation_y (.y _array_element))))
                  (set `local.MaxLocation` (`KismetMathLibrary.MakeVector` (`KismetMathLibrary.FMax` (.x _array_element) _maxlocation_x) (`KismetMathLibrary.FMax` (.y _array_element) _maxlocation_y))))
                (set `local.CenterLocation` (`KismetMathLibrary.TransformLocation` (`self.GetTransform`) (`KismetMathLibrary.MakeVector` (+ (/ (- _maxlocation_x_2 _minlocation_x_2) 2.0) _minlocation_x_2) (+ (/ (- _maxlocation_y_2 _minlocation_y_2) 2.0) _minlocation_y_2)))))))
          (:`then_1`
            ;[1 1 1] Create meshes in triangle
            (`KismetArrayLibrary.Array_Set` _instancedetails _meshindex (make `/Game/MyContent/Blueprints/S_InstanceDetails` "Item") true)
            (set `local.PolyDetailItem` (`|GetArrayItem` _instancedetails _meshindex))
            (set `local.InstanceIndex` 0)
            (for (_array_element_2 _array_index) (`self.Counters`)
              (set `local.MeshCreateIndex` _array_index)
              (bind _returnvalue_5 (`KismetMathLibrary.FTrunc` (+ (* (`KismetMathLibrary.Conv_IntToDouble` _array_element_2) (`local.PercentageThisMesh`)) 0.5)))
              (if (> _returnvalue_5 0)
                (for _ (range (+ _returnvalue_5 1))
                  (bind _point (`self.FindPoint` (`|GetArrayItem` (`self.APoint`) _meshcreateindex) (`|GetArrayItem` (`self.BPoint`) _meshcreateindex) (`|GetArrayItem` (`self.CPoint`) _meshcreateindex))) ; In World Space
                  (set `local.Location` _point)
                  (`|ExecutionSequence`
                    (:`then_0`
                      ;[1 1 1] Setup Rotation
                      (switch `/Game/MyContent/Blueprints/E_RotationType` (`local.Rotation`)
                        (:`NewEnumerator1`
                          (set `local.Rotator` (`KismetMathLibrary.MakeRotator` 0.0 0.0 (`KismetMathLibrary.RandomFloatInRange` 0.0 360.0)) :!label _label))
                        (:`NewEnumerator2`
                          (set `local.Rotator` (`KismetMathLibrary.MakeRotator` _returnvalue_roll_2 _returnvalue_pitch_2 (- _returnvalue_yaw_2 90.0))))
                        (:`NewEnumerator3`
                          (set `local.Rotator` (`KismetMathLibrary.MakeRotator` _returnvalue_roll _returnvalue_pitch (- _returnvalue_yaw 90.0))))
                        (:`NewEnumerator4`
                          (bind _returnvalue_6 (`GameplayStatics.GetActorOfClass` (`self.LookAtActorClass`)))
                          (`/Engine/EditorBlueprintResources/StandardMacros.IsValid` _returnvalue_6
                            (:`Is Valid`
                              (bind (_returnvalue_x_3 _returnvalue_y_3) (`KismetMathLibrary.BreakVector` (`self.K2_GetActorLocation` _returnvalue_6)))
                              (bind (_returnvalue_roll_3 _returnvalue_pitch_3 _returnvalue_yaw_3) (`KismetMathLibrary.BreakRotator` (`KismetMathLibrary.FindLookAtRotation` (`local.Location`) (`KismetMathLibrary.MakeVector` _returnvalue_x_3 _returnvalue_y_3 _returnvalue_z))))
                              (set `local.Rotator` (`KismetMathLibrary.MakeRotator` _returnvalue_roll_3 _returnvalue_pitch_3 (- _returnvalue_yaw_3 90.0))))))
                        (:`NewEnumerator7`
                          (goto _label))))
                    (:`then_1`
                      (bind _returnvalue_7 (`InstancedStaticMeshComponent.AddInstance` (`local.StaticMeshInstance`) (`KismetMathLibrary.MakeTransform` _location _rotator _returnvalue_4) true))
                      (`KismetArrayLibrary.Array_Set` _transform (`local.InstanceIndex`) (`KismetMathLibrary.MakeTransform` _location _rotator _returnvalue_4) true) ; Save Transform
                      (`KismetArrayLibrary.Array_Set` _size (`local.InstanceIndex`) _returnvalue_3 true) ; Save Size as Float
                      (`KismetArrayLibrary.Array_Set` _ratio (`local.InstanceIndex`) (* (/ _returnvalue_3 (`local.Min`)) (`local.GrowthRate`)) true) ; Save Ratio as Float
                      (`/Engine/EditorBlueprintResources/StandardMacros.IncrementInt` (`local.InstanceIndex`)))))))))))))

(fn `FindPoint`
  (params (A :type "Vector Structure") (B :type "Vector Structure") (C :type "Vector Structure"))
  (returns (Point :type "Vector Structure"))
  (locals (R1 :type "Float (double-precision)") (R2 :type "Float (double-precision)"))
  (bind _stream (`self.Stream`))
  (set `local.R1` (`KismetMathLibrary.RandomFloatFromStream` _stream))
  (set `local.R2` (`KismetMathLibrary.RandomFloatFromStream` _stream))
  (return (+ (* A (- 1.0 (`KismetMathLibrary.Sqrt` (`local.R1`)))) (* B (* (`KismetMathLibrary.Sqrt` (`local.R1`)) (- 1.0 (`local.R2`)))) (* C (* (`KismetMathLibrary.Sqrt` (`local.R1`)) (`local.R2`))))))

(fn `Grow and Rotate Instance`
  (params (Layer :type Integer) (InstanceIndex :type Integer))
  (bind _newrotator (`self.NewRotator`))
  (bind (_output_name _output_transform _output_size _output_ratio) (break `/Game/MyContent/Blueprints/S_InstanceDetails` (`|GetArrayItem` (`self.InstanceDetails`) Layer)))
  (bind (_output_staticmesh _output_sizemin _output_sizemax _output_usematerial _output_materialinstance _output_rotationtype _output_lookatlocation _output_percentagethismesh _output_deltainitialsize _output_growthrate _output_hidemeshes) (break `/Game/MyContent/Blueprints/S_PolyDef` (`|GetArrayItem` (`self.MeshLayers`) Layer)))
  (bind (_output_location _output_rotation) (`KismetMathLibrary.BreakTransform` (`|GetArrayItem` _output_transform InstanceIndex)))
  (bind _returnvalue (+ (`|GetArrayItem` _output_size InstanceIndex) (`|GetArrayItem` _output_ratio InstanceIndex)))
  (bind (_returnvalue_roll _returnvalue_pitch _returnvalue_yaw) (`KismetMathLibrary.BreakRotator` (`KismetMathLibrary.FindLookAtRotation` _output_location (`KismetMathLibrary.MakeVector` (.x (`self.ActorLocation`)) (.y (`self.ActorLocation`)) (.z _output_location)))))
  (if (not _output_hidemeshes)
    (if (or (`|EnumEquality` _output_rotationtype "NewEnumerator4") (> _output_growthrate 0.0))
      (set `self.RotationType` _output_rotationtype)
      (if (>= (`KismetArrayLibrary.Array_Length` _output_transform) InstanceIndex)
        (set `self.NewRotator` _output_rotation)
        (`|ExecutionSequence`
          (:`then_0`
            ;[1 1 1] Get look at Rotation
            (if (`|EnumEquality` (`self.RotationType`) "NewEnumerator4")
              (if true
                (set `self.NewRotator` (`KismetMathLibrary.TransformRotation` (`self.GetTransform`) (`KismetMathLibrary.MakeRotator` _returnvalue_roll _returnvalue_pitch (- _returnvalue_yaw 90.0)))))))
          (:`then_1`
            (if (or (< _returnvalue _output_sizemax) (!= _output_rotation _newrotator :`ErrorTolerance` 0.01))
              (`KismetArrayLibrary.Array_Set` _output_size InstanceIndex _returnvalue)
              (`InstancedStaticMeshComponent.UpdateInstanceTransform` (`|GetArrayItem` (`self.InstancedStaticMesh`) Layer) InstanceIndex (`KismetMathLibrary.MakeTransform` _output_location _newrotator (`KismetMathLibrary.Conv_DoubleToVector` _returnvalue)) true true false))))))))

(fn `Grow Next Instance`
  (locals (Counter :type Integer))
  (bind _returnvalue (`KismetArrayLibrary.Array_Length` (`self.MeshLayers`)))
  (bind _returnvalue_2 (`self.K2_GetActorLocation` (`self.LookAtActor`)))
  (if (> _returnvalue 0)
    (for _index (range _returnvalue)
      (`|ExecutionSequence`
        (:`then_0`
          (bind (_output_staticmesh _output_sizemin _output_sizemax _output_usematerial _output_materialinstance _output_rotationtype _output_lookatlocation _output_percentagethismesh _output_deltainitialsize _output_growthrate) (break `/Game/MyContent/Blueprints/S_PolyDef` (`|GetArrayItem` (`self.MeshLayers`) _index)))
          ;[1 1 1] Find look at Actor location
          (if (`|EnumEquality` _output_rotationtype "NewEnumerator4")
            (`|ExecutionSequence`
              (:`then_0`
                (`|DoOnceMultiInput`
                  (:`A Out`
                    (bind _returnvalue_3 (`GameplayStatics.GetActorOfClass` (`self.LookAtActorClass`)))
                    (`/Engine/EditorBlueprintResources/StandardMacros.IsValid` _returnvalue_3
                      (:`Is Valid`
                        (set `self.LookAtActor` _returnvalue_3))
                      (:`Is Not Valid`
                        (set `self.LookAtActor` self))))))
              (:`then_1`
                (set `self.ActorLocationChanged` false)
                (if (!= _returnvalue_2 (`self.ActorLocation`) :`ErrorTolerance` 5.0)
                  (set `self.ActorLocation` _returnvalue_2)
                  (set `self.ActorLocationChanged` true))))))
        (:`then_1`
          (if (> _output_growthrate 0.0)
            (if (not (`self.SmoothGrowth`))
              (bind (_output_name _output_transform) (break `/Game/MyContent/Blueprints/S_InstanceDetails` (`|GetArrayItem` (`self.InstanceDetails`) _index)))
              (bind _returnvalue_4 (- (`KismetArrayLibrary.Array_Length` _output_transform) 1))
              (`self.Grow and Rotate Instance` _index (`KismetMathLibrary.RandomIntegerInRangeFromStream` 0 _returnvalue_4 (`self.Stream`))) ; Grow One Instance per tick
              (else
                (for _index_2 (range (+ _returnvalue_4 1))
                  (`self.Grow and Rotate Instance` _index _index_2) ; Grow All Instances per tick
                )))))))))

(fn `MakeMeshInstance`
  (locals (InstancedMesh :type "InstancedStaticMeshComponent Object Reference"))
  (bind _meshlayers (`self.MeshLayers`))
  (bind _returnvalue (`KismetArrayLibrary.Array_Length` _meshlayers))
  (if (> _returnvalue 0)
    (for _index (range _returnvalue)
      (bind _returnvalue_2 (`AddComponent|NODE_AddInstancedStaticMeshComponent-6`))
      (bind _output_get (set `local.InstancedMesh` _returnvalue_2))
      (`KismetArrayLibrary.Array_Set` (`self.InstancedStaticMesh`) _index _returnvalue_2 true)
      (bind (_output_staticmesh _output_sizemin _output_sizemax _output_usematerial _output_materialinstance) (break `/Game/MyContent/Blueprints/S_PolyDef` (`|GetArrayItem` _meshlayers _index)))
      (`StaticMeshComponent.SetStaticMesh` _output_get _output_staticmesh)
      (`|ExecutionSequence`
        (:`then_0`
          (if _output_usematerial
            (bind _returnvalue_3 (`PrimitiveComponent.CreateDynamicMaterialInstance` (`local.InstancedMesh`) 0 _output_materialinstance "None"))
            (`PrimitiveComponent.SetMaterial` (`local.InstancedMesh`) 0 _returnvalue_3)))))))

(fn `MakeTrianglesFromPolygon`
  (bind _returnvalue (`self.GetTransform`))
  (bind _polygon (`self.Polygon`))
  (bind _returnvalue_2 (`KismetArrayLibrary.Array_Length` (`self.Polygon`)))
  (if (> _returnvalue_2 2)
    (for _index (range 1 (+ (- _returnvalue_2 2) 1))
      (`|ExecutionSequence`
        (:`then_0`
          (bind _returnvalue_3 (- _index 1))
          (`KismetArrayLibrary.Array_Set` (`self.APoint`) _returnvalue_3 (`KismetMathLibrary.TransformLocation` _returnvalue (`|GetArrayItem` _polygon)) true))
        (:`then_1`
          (`KismetArrayLibrary.Array_Set` (`self.BPoint`) _returnvalue_3 (`KismetMathLibrary.TransformLocation` _returnvalue (`|GetArrayItem` _polygon _index)) true))
        (:`then_2`
          (`KismetArrayLibrary.Array_Set` (`self.CPoint`) _returnvalue_3 (`KismetMathLibrary.TransformLocation` _returnvalue (`|GetArrayItem` _polygon (+ _index 1))) true))))))

(fn `SetAreaofTriangle`
  (params (index :type Integer))
  (locals (Triangle :type " Structure") (TIndex :type Integer))
  (bind (_output_x _output_y) (`KismetMathLibrary.BreakVector` (`|GetArrayItem` (`self.APoint`) index)))
  (bind (_output_x_2 _output_y_2) (`KismetMathLibrary.BreakVector` (`|GetArrayItem` (`self.BPoint`) index)))
  (bind (_output_x_3 _output_y_3) (`KismetMathLibrary.BreakVector` (`|GetArrayItem` (`self.CPoint`) index)))
  (bind _returnvalue (`KismetMathLibrary.Sqrt` (+ (`KismetMathLibrary.Square` (- _output_x _output_x_3)) (`KismetMathLibrary.Square` (- _output_y _output_y_3)))))
  (bind _returnvalue_2 (`KismetMathLibrary.Sqrt` (+ (`KismetMathLibrary.Square` (- _output_x_2 _output_x_3)) (`KismetMathLibrary.Square` (- _output_y_2 _output_y_3)))))
  (bind _returnvalue_3 (`KismetMathLibrary.Sqrt` (+ (`KismetMathLibrary.Square` (- _output_x _output_x_2)) (`KismetMathLibrary.Square` (- _output_y _output_y_2)))))
  (set `local.TIndex` index)
  (set `self.A` _returnvalue_3)
  (set `self.B` _returnvalue)
  (set `self.C` _returnvalue_2)
  (set `self.S` (/ (+ _returnvalue_3 _returnvalue _returnvalue_2) 2.0))
  (`KismetArrayLibrary.Array_Set` (`self.Areas`) (`local.TIndex`) (`KismetMathLibrary.Sqrt` (* (`self.S`) (- (`self.S`) (`self.A`)) (- (`self.S`) (`self.B`)) (- (`self.S`) (`self.C`)))) true))

(fn `SetTriangleProperties`
  (locals (AreaIndex :type Integer))
  (`|ExecutionSequence`
    (:`then_0`
      (for (_ _array_index) (`self.APoint`)
        (`self.SetAreaofTriangle` _array_index)))
    (:`then_1`
      (for _array_element (`self.Areas`)
        (set `self.TotalArea` (+ _array_element (`self.TotalArea`)))))
    (:`then_2`
      (for (_array_element_2 _array_index_2) (`self.Areas`)
        (set `local.AreaIndex` _array_index_2)
        (if (> _array_element_2 0.0)
          (bind _returnvalue (/ _array_element_2 (`self.TotalArea`)))
          (`KismetArrayLibrary.Array_Set` (`self.Percentages`) (`local.AreaIndex`) _returnvalue true)
          (`KismetArrayLibrary.Array_Set` (`self.Counters`) (`local.AreaIndex`) (`KismetMathLibrary.FTrunc` (`KismetMathLibrary.FMax` (+ (* _returnvalue (`KismetMathLibrary.Conv_IntToDouble` (`self.TotalEachItems`))) 0.5) 1.0)) true))))))

(fn `ShowDebugOutline`
  (for (_array_element _array_index) (`self.APoint`)
    (`|ExecutionSequence`
      (:`then_0`
        (bind _returnvalue (`KismetMathLibrary.MakeVector` (.x _array_element) (.y _array_element) (+ (.z _array_element) (`self.DebugFenceHeight`))))
        (`KismetSystemLibrary.DrawDebugLine` (`KismetMathLibrary.MakeVector` (.x _array_element) (.y _array_element) (.z _array_element)) _returnvalue (`self.DebugLineColor`) (`self.DebugDuration`) 2.0)
        (`KismetSystemLibrary.DrawDebugCapsule` _returnvalue 0.0 5.0 (struct) (`self.DebugLineColor`) (`self.DebugDuration`) 2.0)
        (bind (_output_x _output_y _output_z) (`KismetMathLibrary.BreakVector` (`|GetArrayItem` (`self.BPoint`) _array_index)))
        (bind _returnvalue_2 (`KismetMathLibrary.MakeVector` _output_x _output_y (+ _output_z (`self.DebugFenceHeight`))))
        (`KismetSystemLibrary.DrawDebugLine` (`KismetMathLibrary.MakeVector` _output_x _output_y _output_z) _returnvalue_2 (`self.DebugLineColor`) (`self.DebugDuration`) 2.0)
        (`KismetSystemLibrary.DrawDebugCapsule` _returnvalue_2 0.0 5.0 (struct) (`self.DebugLineColor`) (`self.DebugDuration`) 2.0)
        (bind (_output_x_2 _output_y_2 _output_z_2) (`KismetMathLibrary.BreakVector` (`|GetArrayItem` (`self.CPoint`) _array_index)))
        (bind _returnvalue_3 (`KismetMathLibrary.MakeVector` _output_x_2 _output_y_2 (+ _output_z_2 (`self.DebugFenceHeight`))))
        (`KismetSystemLibrary.DrawDebugLine` (`KismetMathLibrary.MakeVector` _output_x_2 _output_y_2 _output_z_2) _returnvalue_3 (`self.DebugLineColor`) (`self.DebugDuration`) 2.0)
        (`KismetSystemLibrary.DrawDebugCapsule` _returnvalue_3 0.0 5.0 (struct) (`self.DebugLineColor`) (`self.DebugDuration`) 2.0)
        (`KismetSystemLibrary.DrawDebugLine` _returnvalue _returnvalue_2 (`self.DebugLineColor`) (`self.DebugDuration`) 2.0)
        (`KismetSystemLibrary.DrawDebugLine` _returnvalue_2 _returnvalue_3 (`self.DebugLineColor`) (`self.DebugDuration`) 2.0)
        (`KismetSystemLibrary.DrawDebugLine` _returnvalue _returnvalue_3 (`self.DebugLineColor`) (`self.DebugDuration`) 2.0)))))

(fn `UserConstructionScript`
  (if (`self.UseConstructor`)
    (`|ExecutionSequence`
      (:`then_0`
        (`self.MakeTrianglesFromPolygon`)
        (`self.SetTriangleProperties`)
        (set `self.Stream` (`KismetMathLibrary.MakeRandomStream` (`self.StreamInitialSeed`))))
      (:`then_1`
        (if (`self.ShowDebugFence`)
          (`self.ShowDebugOutline`)))
      (:`then_2`
        (if (not (`self.HideMeshes`))
          (`self.MakeMeshInstance`)
          (`self.FillTrianglesWithMeshes`))))))