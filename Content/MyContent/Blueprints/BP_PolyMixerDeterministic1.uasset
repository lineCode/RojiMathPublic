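; Actor that scatters weighted layers of instanced static meshes inside a polygon, with an optional debug fence.
; Fan-triangulates Points, splitting item counts by Heron-formula area.
; Seeded barycentric sampling places and sizes instances per PolyDefs layer with selectable rotation modes, though Random yaw is unseeded.
; Builds in construction or at BeginPlay via UseConstructor; timers redraw the fence, grow instances and turn them toward a tracked actor.
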(event `self.ReceiveBeginPlay`
  (if (not (`self.UseConstructor`))
    (`KismetSystemLibrary.Delay` 0.2)
    (`|ExecutionSequence`
      (:`then_0`
        ;[1 1 1] Create Triangles from Polygon and set area, percentage and count
        (`self.MakeTrianglesFromPolygon`)
        (`self.SetTriangleProperties`))
      (:`then_1`
        ;[1 1 1] Show Debug Fence
        (if (`self.ShowDebugFence`)
          (`self.ShowDebugOutline`)))
      (:`then_2`
        ;[1 1 1] Make the Mesh Instances and individual Meshes in the Triangles
        (if (not (`self.HideMeshes`))
          (`self.MakeMeshInstance`)
          (`self.FillTrianglesWithMeshes`)))
      (:`then_3`
        ;[1 1 1] Start timers for updating Debug Fence and Mesh Manipulation over time
        (`KismetSystemLibrary.K2_SetTimerDelegate` (delegate `UpdateDebugFence`) (`self.DebugDuration`) true :!label _label)
        (`KismetSystemLibrary.K2_SetTimerDelegate` (delegate `GrowInstance`) 0.041667 (`self.UseTimers`))))
    (else
      (goto _label))))

(event `UpdateDebugFence`
  (if (`self.ShowDebugFence`)
    (`self.ShowDebugOutline`)))

(event `GrowInstance`
  (`self.GrowNow1`))

(fn `FillTrianglesWithMeshes`
  (locals (Rotator :type "Rotator Structure" :default (struct)) (Location :type "Vector Structure" :default (0.0 0.0 0.0)) (CenterLocation :type "Vector Structure") (MinLocation :type "Vector Structure") (MaxLocation :type "Vector Structure") (Min :type "Float (double-precision)") (Max :type "Float (double-precision)") (LookLocation :type "Vector Structure") (ScaleSize :type "Float (double-precision)") (StaticMeshInstance :type "InstancedStaticMeshComponent Object Reference") (Rotation :type "/Game/MyContent/Blueprints/E_RotationType Enum") (PercentageThisMesh :type "Float (double-precision)") (MeshIndex :type Integer) (PolyDetailItem :type "/Game/MyContent/Blueprints/S_InstanceDetails Structure") (MeshCreateIndex :type Integer) (InstanceIndex :type Integer) (DeltaInitialSize :type "Float (double-precision)") (GrowthRate :type "Float (double-precision)"))
  (bind (_returnvalue_x _returnvalue_y _returnvalue_z) (`KismetMathLibrary.BreakVector` (`self.K2_GetActorLocation`)))
  (bind (_returnvalue_x_2 _returnvalue_y_2 _returnvalue_z_2) (`KismetMathLibrary.BreakVector` (`self.K2_GetActorLocation`)))
  (bind (_minlocation_x _minlocation_y) (`KismetMathLibrary.BreakVector` (`local.MinLocation`)))
  (bind (_maxlocation_x _maxlocation_y) (`KismetMathLibrary.BreakVector` (`local.MaxLocation`)))
  (bind _points (`self.Points`))
  (bind (_looklocation_x _looklocation_y) (`KismetMathLibrary.BreakVector` (`local.LookLocation`)))
  (bind _rotator (`local.Rotator`))
  (bind _instancedetails (`self.InstanceDetails`))
  (bind _meshindex (`local.MeshIndex`))
  (bind _location (`local.Location`))
  (bind (_minlocation_x_2 _minlocation_y_2) (`KismetMathLibrary.BreakVector` (`local.MinLocation`)))
  (bind (_maxlocation_x_2 _maxlocation_y_2) (`KismetMathLibrary.BreakVector` (`local.MaxLocation`)))
  (bind _returnvalue (`KismetArrayLibrary.Array_Length` (`self.InstancedStaticMesh`)))
  (bind (_returnvalue_roll _returnvalue_pitch _returnvalue_yaw) (`KismetMathLibrary.BreakRotator` (`KismetMathLibrary.FindLookAtRotation` (`local.Location`) (`local.CenterLocation`))))
  (bind (_output_staticmesh _output_sizemin _output_sizemax _output_usematerial _output_materialinstance _output_rotationtype _output_lookatlocation _output_percentagethismesh _output_deltainitialsize _output_growthrate _output_hidemeshes) (break `/Game/MyContent/Blueprints/S_PolyDef` (`|GetArrayItem` (`self.PolyDefs`) (`local.MeshIndex`))))
  (bind _output (`|GetArrayItem` _points))
  (bind _returnvalue_2 (* (`local.Min`) (`local.DeltaInitialSize`)))
  (bind (_name _transform _size _ratio) (break `/Game/MyContent/Blueprints/S_InstanceDetails` (`|GetArrayItem` (`self.InstanceDetails`) (`local.MeshIndex`))))
  (bind (_returnvalue_roll_2 _returnvalue_pitch_2 _returnvalue_yaw_2) (`KismetMathLibrary.BreakRotator` (`KismetMathLibrary.FindLookAtRotation` (`local.Location`) (`KismetMathLibrary.MakeVector` _looklocation_x _looklocation_y _returnvalue_z_2))))
  (bind _returnvalue_3 (`KismetMathLibrary.RandomFloatInRangeFromStream` (- (`local.Min`) _returnvalue_2) (+ (`local.Min`) _returnvalue_2) (`self.Stream`)))
  (bind _returnvalue_4 (`KismetMathLibrary.Conv_DoubleToVector` _returnvalue_3))
  ;[1 1 1] Setup
  (if (> _returnvalue 0)
    (for _index (range _returnvalue)
      (set `local.MeshIndex` _index)
      (set `local.StaticMeshInstance` (`|GetArrayItem` (`self.InstancedStaticMesh`) (`local.MeshIndex`)))
      (if (not _output_hidemeshes)
        (set `local.Min` _output_sizemin)
        (set `local.Rotation` _output_rotationtype)
        (set `local.Max` _output_sizemax)
        (set `local.LookLocation` _output_lookatlocation)
        (set `local.PercentageThisMesh` _output_percentagethismesh)
        (set `local.DeltaInitialSize` _output_deltainitialsize)
        (set `local.GrowthRate` _output_growthrate)
        (`|ExecutionSequence`
          (:`then_0`
            ;[1 1 1] Find "Center" of polygon
            (if (`|EnumEquality` (`local.Rotation`) "NewEnumerator3")
              (if (> (`KismetArrayLibrary.Array_Length` _points) 0)
                (set `local.MinLocation` _output)
                (set `local.MaxLocation` _output)
                (for _array_element (`self.Points`)
                  (set `local.MinLocation` (`KismetMathLibrary.MakeVector` (`KismetMathLibrary.FMin` _minlocation_x (.x _array_element)) (`KismetMathLibrary.FMin` _minlocation_y (.y _array_element))))
                  (set `local.MaxLocation` (`KismetMathLibrary.MakeVector` (`KismetMathLibrary.FMax` (.x _array_element) _maxlocation_x) (`KismetMathLibrary.FMax` (.y _array_element) _maxlocation_y))))
                (set `local.CenterLocation` (`KismetMathLibrary.TransformLocation` (`self.GetTransform`) (`KismetMathLibrary.MakeVector` (+ (/ (- _maxlocation_x_2 _minlocation_x_2) 2.0) _minlocation_x_2) (+ (/ (- _maxlocation_y_2 _minlocation_y_2) 2.0) _minlocation_y_2)))))))
          (:`then_1`
            ;[1 1 1] Create meshes in triangle
            (`KismetArrayLibrary.Array_Set` _instancedetails _meshindex (make `/Game/MyContent/Blueprints/S_InstanceDetails` "Item") true)
            (set `local.PolyDetailItem` (`|GetArrayItem` _instancedetails _meshindex))
            (set `local.InstanceIndex` 0)
            (for (_array_element_2 _array_index) (`self.Counters`)
              (set `local.MeshCreateIndex` _array_index)
              (bind _returnvalue_5 (`KismetMathLibrary.FTrunc` (+ (* (`KismetMathLibrary.Conv_IntToDouble` _array_element_2) (`local.PercentageThisMesh`)) 0.5)))
              (if (> _returnvalue_5 0)
                (for _ (range (+ _returnvalue_5 1))
                  (bind _point (`self.FindPoint` (`|GetArrayItem` (`self.Triangles`) (`local.MeshCreateIndex`)))) ; In World Space
                  (set `local.Location` _point)
                  (`|ExecutionSequence`
                    (:`then_0`
                      ;[1 1 1] Setup Rotation
                      (switch `/Game/MyContent/Blueprints/E_RotationType` (`local.Rotation`)
                        (:`NewEnumerator8`
                          (set `local.Rotator` (struct) :!label _label))
                        (:`NewEnumerator5`
                          (goto _label))
                        (:`NewEnumerator9`
                          (goto _label))
                        (:`NewEnumerator1`
                          (set `local.Rotator` (`KismetMathLibrary.MakeRotator` 0.0 0.0 (`KismetMathLibrary.RandomFloatInRange` 0.0 360.0))))
                        (:`NewEnumerator2`
                          (set `local.Rotator` (`KismetMathLibrary.MakeRotator` _returnvalue_roll_2 _returnvalue_pitch_2 (- _returnvalue_yaw_2 90.0))))
                        (:`NewEnumerator3`
                          (set `local.Rotator` (`KismetMathLibrary.MakeRotator` _returnvalue_roll _returnvalue_pitch (- _returnvalue_yaw 90.0))))
                        (:`NewEnumerator4`
                          (bind _returnvalue_6 (`GameplayStatics.GetActorOfClass` (`self.LookActorClass`)))
                          (`/Engine/EditorBlueprintResources/StandardMacros.IsValid` _returnvalue_6
                            (:`Is Valid`
                              (bind (_returnvalue_x_3 _returnvalue_y_3) (`KismetMathLibrary.BreakVector` (`self.K2_GetActorLocation` _returnvalue_6)))
                              (bind (_returnvalue_roll_3 _returnvalue_pitch_3 _returnvalue_yaw_3) (`KismetMathLibrary.BreakRotator` (`KismetMathLibrary.FindLookAtRotation` (`local.Location`) (`KismetMathLibrary.MakeVector` _returnvalue_x_3 _returnvalue_y_3 _returnvalue_z))))
                              (set `local.Rotator` (`KismetMathLibrary.MakeRotator` _returnvalue_roll_3 _returnvalue_pitch_3 (- _returnvalue_yaw_3 90.0))))))))
                    (:`then_1`
                      (bind _returnvalue_7 (`InstancedStaticMeshComponent.AddInstance` (`local.StaticMeshInstance`) (`KismetMathLibrary.MakeTransform` _location _rotator _returnvalue_4) true))
                      (`KismetArrayLibrary.Array_Set` _transform (`local.InstanceIndex`) (`KismetMathLibrary.MakeTransform` _location _rotator _returnvalue_4) true) ; Save Transform
                      (`KismetArrayLibrary.Array_Set` _size (`local.InstanceIndex`) _returnvalue_3 true) ; Save Size as Float
                      (`KismetArrayLibrary.Array_Set` _ratio (`local.InstanceIndex`) (* (/ _returnvalue_3 (`local.Min`)) (`local.GrowthRate`)) true) ; Save Ratio as Float
                      (`/Engine/EditorBlueprintResources/StandardMacros.IncrementInt` (`local.InstanceIndex`)))))))))))))

(fn `FindPoint`
  (params (Triangle :type "/Game/MyContent/Blueprints/S_Triangle Structure"))
  (returns (Point :type "Vector Structure"))
  (locals (lTriangle :type "/Game/MyContent/Blueprints/S_Triangle Structure") (R1 :type "Float (double-precision)") (R2 :type "Float (double-precision)"))
  (bind _stream (`self.Stream`))
  (bind (_ltriangle_a _ltriangle_b _ltriangle_c) (break `/Game/MyContent/Blueprints/S_Triangle` (`local.lTriangle`)))
  (set `local.lTriangle` Triangle)
  (set `local.R1` (`KismetMathLibrary.RandomFloatFromStream` _stream))
  (set `local.R2` (`KismetMathLibrary.RandomFloatFromStream` _stream))
  (return (+ (* _ltriangle_a (- 1.0 (`KismetMathLibrary.Sqrt` (`local.R1`)))) (* _ltriangle_b (* (`KismetMathLibrary.Sqrt` (`local.R1`)) (- 1.0 (`local.R2`)))) (* _ltriangle_c (* (`KismetMathLibrary.Sqrt` (`local.R1`)) (`local.R2`))))))

(fn `GrowNow1`
  (locals (Counter :type Integer))
  (bind _newrotator (`self.NewRotator`))
  (bind _returnvalue (`KismetArrayLibrary.Array_Length` (`self.PolyDefs`)))
  (bind _returnvalue_2 (`self.K2_GetActorLocation` (`self.LookAtActor`)))
  (if (> _returnvalue 0)
    (for _index (range _returnvalue)
      (bind (_output_staticmesh _output_sizemin _output_sizemax _output_usematerial _output_materialinstance _output_rotationtype _output_lookatlocation _output_percentagethismesh _output_deltainitialsize _output_growthrate _output_hidemeshes) (break `/Game/MyContent/Blueprints/S_PolyDef` (`|GetArrayItem` (`self.PolyDefs`) _index)))
      (if (not _output_hidemeshes)
        (if (or (`|EnumEquality` _output_rotationtype "NewEnumerator4") (> _output_growthrate 0.0))
          (set `self.RotationType` _output_rotationtype)
          (`|ExecutionSequence`
            (:`then_0`
              ;[1 1 1] Find look at Actor location
              (if (`|EnumEquality` (`self.RotationType`) "NewEnumerator4")
                (`|ExecutionSequence`
                  (:`then_0`
                    (`|DoOnceMultiInput`
                      (:`A Out`
                        (bind _returnvalue_3 (`GameplayStatics.GetActorOfClass` (`self.LookActorClass`)))
                        (`/Engine/EditorBlueprintResources/StandardMacros.IsValid` _returnvalue_3
                          (:`Is Valid`
                            (set `self.LookAtActor` _returnvalue_3))
                          (:`Is Not Valid`
                            (set `self.LookAtActor` self))))))
                  (:`then_1`
                    (set `self.ActorLocationChanged` false)
                    (if (!= _returnvalue_2 (`self.ActorLocation`) :`ErrorTolerance` 5.0)
                      (set `self.ActorLocation` _returnvalue_2)
                      (set `self.ActorLocationChanged` true))))))
            (:`then_2`
              (bind (_output_name _output_transform _output_size _output_ratio) (break `/Game/MyContent/Blueprints/S_InstanceDetails` (`|GetArrayItem` (`self.InstanceDetails`) _index)))
              (for (_array_element _array_index) _output_transform
                (set `self.NewRotator` (.rotation _array_element))
                (`|ExecutionSequence`
                  (:`then_0`
                    ;[1 1 1] Get look at Rotation
                    (if (`|EnumEquality` (`self.RotationType`) "NewEnumerator4")
                      (if (`self.ActorLocationChanged`)
                        (bind _output_location (`KismetMathLibrary.BreakTransform` (`|GetArrayItem` _output_transform (`local.Counter`))))
                        (bind (_returnvalue_roll _returnvalue_pitch _returnvalue_yaw) (`KismetMathLibrary.BreakRotator` (`KismetMathLibrary.FindLookAtRotation` _output_location (`self.ActorLocation`))))
                        (set `self.NewRotator` (`KismetMathLibrary.TransformRotation` (`self.GetTransform`) (`KismetMathLibrary.MakeRotator` _returnvalue_roll _returnvalue_pitch (- _returnvalue_yaw 90.0)))))))
                  (:`then_1`
                    (bind _returnvalue_4 (+ (`|GetArrayItem` _output_size _array_index) (`|GetArrayItem` _output_ratio _array_index)))
                    (if (or (< _returnvalue_4 _output_sizemax) (!= (.rotation _array_element) _newrotator :`ErrorTolerance` 0.01))
                      (`KismetArrayLibrary.Array_Set` _output_size _array_index _returnvalue_4)
                      (`InstancedStaticMeshComponent.UpdateInstanceTransform` (`|GetArrayItem` (`self.InstancedStaticMesh`) _index) _array_index (`KismetMathLibrary.MakeTransform` _output_location _newrotator (`KismetMathLibrary.Conv_DoubleToVector` _returnvalue_4)) true true false))))))))))))

(fn `MakeMeshInstance`
  (locals (InstancedMesh :type "InstancedStaticMeshComponent Object Reference"))
  (bind _polydefs (`self.PolyDefs`))
  (bind _returnvalue (`KismetArrayLibrary.Array_Length` _polydefs))
  (if (> _returnvalue 0)
    (for _index (range _returnvalue)
      (bind _returnvalue_2 (`AddComponent|NODE_AddInstancedStaticMeshComponent-6`))
      (bind _output_get (set `local.InstancedMesh` _returnvalue_2))
      (`KismetArrayLibrary.Array_Set` (`self.InstancedStaticMesh`) _index _returnvalue_2 true)
      (bind (_output_staticmesh _output_sizemin _output_sizemax _output_usematerial _output_materialinstance) (break `/Game/MyContent/Blueprints/S_PolyDef` (`|GetArrayItem` _polydefs _index)))
      (`StaticMeshComponent.SetStaticMesh` _output_get _output_staticmesh)
      (`|ExecutionSequence`
        (:`then_0`
          (if _output_usematerial
            (bind _returnvalue_3 (`PrimitiveComponent.CreateDynamicMaterialInstance` (`local.InstancedMesh`) 0 _output_materialinstance "None"))
            (`PrimitiveComponent.SetMaterial` (`local.InstancedMesh`) 0 _returnvalue_3)))))))

(fn `MakeTrianglesFromPolygon`
  (bind _returnvalue (`self.GetTransform`))
  (bind _points (`self.Points`))
  (bind _returnvalue_2 (`KismetArrayLibrary.Array_Length` (`self.Points`)))
  (if (> _returnvalue_2 2)
    (for _index (range 1 (+ (- _returnvalue_2 2) 1))
      (`KismetArrayLibrary.Array_Set` (`self.Triangles`) _index (make `/Game/MyContent/Blueprints/S_Triangle` (`KismetMathLibrary.TransformLocation` _returnvalue (`|GetArrayItem` _points)) (`KismetMathLibrary.TransformLocation` _returnvalue (`|GetArrayItem` _points _index)) (`KismetMathLibrary.TransformLocation` _returnvalue (`|GetArrayItem` _points (+ _index 1)))) true))))

(fn `SetAreaofTriangle`
  (params (index :type Integer))
  (locals (Triangle :type "/Game/MyContent/Blueprints/S_Triangle Structure") (TIndex :type Integer))
  (set `local.TIndex` index)
  (bind _output_get (set `local.Triangle` (`|GetArrayItem` (`self.Triangles`) index))) ; heron's formula
  (bind _returnvalue (`KismetMathLibrary.Sqrt` (+ (`KismetMathLibrary.Square` (- (.x (break `/Game/MyContent/Blueprints/S_Triangle` _output_get)) (.x (`.B_5_7713A53B486C6F4EF10E45A452CF54A8` (break `/Game/MyContent/Blueprints/S_Triangle` _output_get))))) (`KismetMathLibrary.Square` (- (.y (break `/Game/MyContent/Blueprints/S_Triangle` _output_get)) (.y (`.B_5_7713A53B486C6F4EF10E45A452CF54A8` (break `/Game/MyContent/Blueprints/S_Triangle` _output_get))))))))
  (set `self.A` _returnvalue)
  (bind _returnvalue_2 (`KismetMathLibrary.Sqrt` (+ (`KismetMathLibrary.Square` (- (.x (break `/Game/MyContent/Blueprints/S_Triangle` _output_get)) (.x (`.C_6_A8CB31CC42EAD84629085288A291D1BE` (break `/Game/MyContent/Blueprints/S_Triangle` _output_get))))) (`KismetMathLibrary.Square` (- (.y (break `/Game/MyContent/Blueprints/S_Triangle` _output_get)) (.y (`.C_6_A8CB31CC42EAD84629085288A291D1BE` (break `/Game/MyContent/Blueprints/S_Triangle` _output_get))))))))
  (set `self.B` _returnvalue_2)
  (bind _returnvalue_3 (`KismetMathLibrary.Sqrt` (+ (`KismetMathLibrary.Square` (- (.x (`.B_5_7713A53B486C6F4EF10E45A452CF54A8` (break `/Game/MyContent/Blueprints/S_Triangle` _output_get))) (.x (`.C_6_A8CB31CC42EAD84629085288A291D1BE` (break `/Game/MyContent/Blueprints/S_Triangle` _output_get))))) (`KismetMathLibrary.Square` (- (.y (`.B_5_7713A53B486C6F4EF10E45A452CF54A8` (break `/Game/MyContent/Blueprints/S_Triangle` _output_get))) (.y (`.C_6_A8CB31CC42EAD84629085288A291D1BE` (break `/Game/MyContent/Blueprints/S_Triangle` _output_get))))))))
  (set `self.C` _returnvalue_3)
  (set `self.S` (/ (+ _returnvalue _returnvalue_2 _returnvalue_3) 2.0))
  (`KismetArrayLibrary.Array_Set` (`self.Areas`) (`local.TIndex`) (`KismetMathLibrary.Sqrt` (* (`self.S`) (- (`self.S`) (`self.A`)) (- (`self.S`) (`self.B`)) (- (`self.S`) (`self.C`)))) true))

(fn `SetTriangleProperties`
  (locals (AreaIndex :type Integer))
  (`|ExecutionSequence`
    (:`then_0`
      (for (_ _array_index) (`self.Triangles`)
        (`self.SetAreaofTriangle` _array_index)))
    (:`then_1`
      (for _array_element (`self.Areas`)
        (set `self.TotalArea` (+ _array_element (`self.TotalArea`)))))
    (:`then_2`
      (for (_array_element_2 _array_index_2) (`self.Areas`)
        (set `local.AreaIndex` _array_index_2)
        (if (> _array_element_2 0.0)
          (bind _returnvalue (/ _array_element_2 (`self.TotalArea`)))
          (`KismetArrayLibrary.Array_Set` (`self.Percentages`) (`local.AreaIndex`) _returnvalue true)
          (`KismetArrayLibrary.Array_Set` (`self.Counters`) (`local.AreaIndex`) (`KismetMathLibrary.FTrunc` (`KismetMathLibrary.FMax` (+ (* _returnvalue (`KismetMathLibrary.Conv_IntToDouble` (`self.TotalEachItems`))) 0.5) 1.0)) true))))))

(fn `ShowDebugOutline`
  (for _array_element (`self.Triangles`)
    (`|ExecutionSequence`
      (:`then_0`
        (bind _returnvalue (`KismetMathLibrary.MakeVector` (.x (break `/Game/MyContent/Blueprints/S_Triangle` _array_element)) (.y (break `/Game/MyContent/Blueprints/S_Triangle` _array_element)) (+ (.z (break `/Game/MyContent/Blueprints/S_Triangle` _array_element)) (`self.DebugFenceHeight`))))
        (`KismetSystemLibrary.DrawDebugLine` (`KismetMathLibrary.MakeVector` (.x (break `/Game/MyContent/Blueprints/S_Triangle` _array_element)) (.y (break `/Game/MyContent/Blueprints/S_Triangle` _array_element)) (.z (break `/Game/MyContent/Blueprints/S_Triangle` _array_element))) _returnvalue (`self.DebugLineColor`) (`self.DebugDuration`) 2.0)
        (`KismetSystemLibrary.DrawDebugCapsule` _returnvalue 0.0 5.0 (struct) (`self.DebugLineColor`) (`self.DebugDuration`) 2.0)
        (bind _returnvalue_2 (`KismetMathLibrary.MakeVector` (.x (`.B_5_7713A53B486C6F4EF10E45A452CF54A8` (break `/Game/MyContent/Blueprints/S_Triangle` _array_element))) (.y (`.B_5_7713A53B486C6F4EF10E45A452CF54A8` (break `/Game/MyContent/Blueprints/S_Triangle` _array_element))) (+ (.z (`.B_5_7713A53B486C6F4EF10E45A452CF54A8` (break `/Game/MyContent/Blueprints/S_Triangle` _array_element))) (`self.DebugFenceHeight`))))
        (`KismetSystemLibrary.DrawDebugLine` (`KismetMathLibrary.MakeVector` (.x (`.B_5_7713A53B486C6F4EF10E45A452CF54A8` (break `/Game/MyContent/Blueprints/S_Triangle` _array_element))) (.y (`.B_5_7713A53B486C6F4EF10E45A452CF54A8` (break `/Game/MyContent/Blueprints/S_Triangle` _array_element))) (.z (`.B_5_7713A53B486C6F4EF10E45A452CF54A8` (break `/Game/MyContent/Blueprints/S_Triangle` _array_element)))) _returnvalue_2 (`self.DebugLineColor`) (`self.DebugDuration`) 2.0)
        (`KismetSystemLibrary.DrawDebugCapsule` _returnvalue_2 0.0 5.0 (struct) (`self.DebugLineColor`) (`self.DebugDuration`) 2.0)
        (bind _returnvalue_3 (`KismetMathLibrary.MakeVector` (.x (`.C_6_A8CB31CC42EAD84629085288A291D1BE` (break `/Game/MyContent/Blueprints/S_Triangle` _array_element))) (.y (`.C_6_A8CB31CC42EAD84629085288A291D1BE` (break `/Game/MyContent/Blueprints/S_Triangle` _array_element))) (+ (.z (`.C_6_A8CB31CC42EAD84629085288A291D1BE` (break `/Game/MyContent/Blueprints/S_Triangle` _array_element))) (`self.DebugFenceHeight`))))
        (`KismetSystemLibrary.DrawDebugLine` (`KismetMathLibrary.MakeVector` (.x (`.C_6_A8CB31CC42EAD84629085288A291D1BE` (break `/Game/MyContent/Blueprints/S_Triangle` _array_element))) (.y (`.C_6_A8CB31CC42EAD84629085288A291D1BE` (break `/Game/MyContent/Blueprints/S_Triangle` _array_element))) (.z (`.C_6_A8CB31CC42EAD84629085288A291D1BE` (break `/Game/MyContent/Blueprints/S_Triangle` _array_element)))) _returnvalue_3 (`self.DebugLineColor`) (`self.DebugDuration`) 2.0)
        (`KismetSystemLibrary.DrawDebugCapsule` _returnvalue_3 0.0 5.0 (struct) (`self.DebugLineColor`) (`self.DebugDuration`) 2.0)
        (`KismetSystemLibrary.DrawDebugLine` _returnvalue _returnvalue_2 (`self.DebugLineColor`) (`self.DebugDuration`) 2.0)
        (`KismetSystemLibrary.DrawDebugLine` _returnvalue_2 _returnvalue_3 (`self.DebugLineColor`) (`self.DebugDuration`) 2.0)
        (`KismetSystemLibrary.DrawDebugLine` _returnvalue _returnvalue_3 (`self.DebugLineColor`) (`self.DebugDuration`) 2.0)))))

(fn `UserConstructionScript`
  (if (`self.UseConstructor`)
    (`|ExecutionSequence`
      (:`then_0`
        (`self.MakeTrianglesFromPolygon`)
        (`self.SetTriangleProperties`))
      (:`then_1`
        (if (`self.ShowDebugFence`)
          (`self.ShowDebugOutline`)))
      (:`then_2`
        (if (not (`self.HideMeshes`))
          (`self.MakeMeshInstance`)
          (`self.FillTrianglesWithMeshes`))))))